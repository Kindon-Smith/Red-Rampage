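; Player marine pawn with world-axis movement, twin-stick style aiming and cosmetic weapon firing.
; Each tick it sets control rotation yaw from gamepad thumbstick direction or interpolated mouse velocity direction, only when input exceeds a deadzone threshold.
; Any key press switches aim mode by checking whether it is a gamepad key.
; Fire input toggles the rifle muzzle-flash particles and looping sound, playing an end sound on release.
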(event `InputAxis|MoveForward`
  (params (AxisValue :type "Float (single-precision)"))
  (`self.AddMovementInput` (1.0 0.0 0.0) AxisValue))

(event `InputAction|Fire Weapon`
  (params (Key :type "Key Structure"))
  (:`Pressed`
    (`self.Start Firing Weapon`))
  (:`Released`
    (`self.Stop Firing Weapon`)))

(event `InputAxis|MoveRight`
  (params (AxisValue :type "Float (single-precision)"))
  (`self.AddMovementInput` (0.0 1.0 0.0) AxisValue))

(event `self.ReceiveTick`
  (params (DeltaSeconds :type "Float (single-precision)"))
  (`self.Update Player Aim`))

(event `Key|AnyKey`
  (params (Key :type "Key Structure"))
  (:`Pressed`
    (set `self.Is Gamepad Active` (`KismetInputLibrary.Key_IsGamepadKey` Key))))

(fn `Get Mouse Aim Direction`
  (returns (ReturnValue :type "Rotator Structure"))
  (bind (_returnvalue_x _returnvalue_y) (`KismetMathLibrary.BreakVector2D` (`self.Get Mouse Velocity`)))
  (return (`KismetMathLibrary.RInterpTo` (`Controller.GetControlRotation` (`GameplayStatics.GetPlayerController` 0)) (`KismetMathLibrary.MakeRotator` 0.0 0.0 (`KismetMathLibrary.DegAtan2` _returnvalue_x _returnvalue_y)) (`GameplayStatics.GetWorldDeltaSeconds`) (`self.Mouse Smoothing Strength`))))

(fn `Get Mouse Velocity`
  (returns (ReturnValue :type "Vector2D Structure"))
  (bind (_deltax _deltay) (`PlayerController.GetInputMouseDelta` (`GameplayStatics.GetPlayerController` 0)))
  (return (/ (`KismetMathLibrary.MakeVector2D` _deltax _deltay) (`GameplayStatics.GetWorldDeltaSeconds`))))

(fn `Get Tumbstick Aim Direction`
  (returns (ReturnValue2 :type "Rotator Structure"))
  (return (`KismetMathLibrary.MakeRotator` 0.0 0.0 (`KismetMathLibrary.DegAtan2` (`self.GetInputAxisValue`) (`self.GetInputAxisValue`)))))

(fn `Is Mouse Deadzone`
  (returns (MouseAlive :type Boolean))
  (return (> (`KismetMathLibrary.VSize2D` (`self.Get Mouse Velocity`)) (`self.Mouse Deadzone Value`))))

(fn `Is Thumbstick Deadzone`
  (returns (`Thumbstick Dead` :type Boolean))
  (return (> (`KismetMathLibrary.VSize2D` (`KismetMathLibrary.MakeVector2D` (`self.GetInputAxisValue`) (`self.GetInputAxisValue`))) (`self.Thumbstick Deadzone Value`))))

(fn `Start Firing Weapon`
  (`ActorComponent.Activate` (`self.P_AssaultRifle_MF`) false)
  (bind _returnvalue (`GameplayStatics.SpawnSound2D` "/Game/Sounds/Weapon_AssaultRifle/Stereo/rifleFireLoop_Cue.rifleFireLoop_Cue" 1.0 1.0 0.0 null))
  (set `self.Weapon Fire Sound` _returnvalue))

(fn `Stop Firing Weapon`
  (`ActorComponent.Deactivate` (`self.P_AssaultRifle_MF`))
  (`AudioComponent.Stop` (`self.Weapon Fire Sound`))
  (`GameplayStatics.SpawnSound2D` "/Game/Sounds/Weapon_AssaultRifle/Stereo/RifleFireEnd_Cue.RifleFireEnd_Cue" 1.0 1.0 0.0 null))

(fn `Update Mouse Aim`
  (if (`self.Is Mouse Deadzone`)
    (`Controller.SetControlRotation` (`GameplayStatics.GetPlayerController` 0) (`self.Get Mouse Aim Direction`))))

(fn `Update Player Aim`
  (if (`self.Is Gamepad Active`)
    (`self.Update Thumbstick Aim`)
    (else
      (`self.Update Mouse Aim`))))

(fn `Update Thumbstick Aim`
  (if (`self.Is Thumbstick Deadzone`)
    (`Controller.SetControlRotation` (`GameplayStatics.GetPlayerController` 0) (`self.Get Tumbstick Aim Direction`))))

(fn `UserConstructionScript`)